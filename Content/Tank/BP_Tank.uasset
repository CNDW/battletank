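; Player-controllable tank Blueprint that wires input and components to movement, aiming and track logic.
; BeginPlay initializes TankMovement with both tracks and TankAiming with the barrel and turret, and track hit events are forwarded to each track's OnHit.
; Input supports direct per-track throttle or forward/turn intents through TankMovement, frame-rate-scaled camera aim via an azimuth gimbal and spring arm, and firing through TankAiming.
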(event `self.ReceiveBeginPlay`
  (`TankMovementComponent.Initialize` (`self.TankMovement`) (`self.TankTrackLeft`) (`self.TankTrackRight`))
  (`TankAimingComponent.Initialize` (`self.TankAiming`) (`self.TankBarrel`) (`self.TankTurret`)))

(event `self.TankTrackRight.OnComponentHit`
  (params (HitComponent :type "PrimitiveComponent Object Reference") (OtherActor :type "Actor Object Reference") (OtherComp :type "PrimitiveComponent Object Reference") (NormalImpulse :type "Vector Structure") (Hit :type "HitResult Structure (by ref)"))
  (`TankTrackComponent.OnHit` (`self.TankTrackRight`) HitComponent OtherActor OtherComp NormalImpulse Hit))

(event `self.TankTrackLeft.OnComponentHit`
  (params (HitComponent :type "PrimitiveComponent Object Reference") (OtherActor :type "Actor Object Reference") (OtherComp :type "PrimitiveComponent Object Reference") (NormalImpulse :type "Vector Structure") (Hit :type "HitResult Structure (by ref)"))
  (`TankTrackComponent.OnHit` (`self.TankTrackLeft`) HitComponent OtherActor OtherComp NormalImpulse Hit))

(event `InputAxis|AimZenith`
  (params (AxisValue :type "Float (single-precision)"))
  ;[1 1 1] Aim Input bindings
  (`SceneComponent.K2_AddLocalRotation` (`self.SpringArm`) (`KismetMathLibrary.MakeRotator` 0.0 (* AxisValue (`GameplayStatics.GetWorldDeltaSeconds`) 100.0)) false false))

(event `InputAxis|Left Track Throttle`
  (params (AxisValue :type "Float (single-precision)"))
  ;[1 1 1] Movement Bindings
  (`TankTrackComponent.SetThrottle` (`self.TankTrackLeft`) AxisValue))

(event `InputAxis|Right Track Throttle`
  (params (AxisValue :type "Float (single-precision)"))
  ;[1 1 1] Movement Bindings
  (`TankTrackComponent.SetThrottle` (`self.TankTrackRight`) AxisValue))

(event `InputAxis|AimAzimuth`
  (params (AxisValue :type "Float (single-precision)"))
  ;[1 1 1] Aim Input bindings
  (`SceneComponent.K2_AddLocalRotation` (`self.AzimuthGimble`) (`KismetMathLibrary.MakeRotator` 0.0 0.0 (* AxisValue (`GameplayStatics.GetWorldDeltaSeconds`) 100.0)) false false))

(event `InputAxis|Tank Forward`
  (params (AxisValue :type "Float (single-precision)"))
  ;[1 1 1] Movement Bindings
  (`TankMovementComponent.IntendMoveForward` (`self.TankMovement`) AxisValue))

(event `InputAxis|Tank Turn Right`
  (params (AxisValue :type "Float (single-precision)"))
  ;[1 1 1] Movement Bindings
  (`TankMovementComponent.IntentTurnRight` (`self.TankMovement`) AxisValue))

(event `InputAction|Fire`
  (params (Key :type "Key Structure"))
  ;[1 1 1] Aim Input bindings
  (:`Pressed`
    (`TankAimingComponent.Fire` (`self.TankAiming`))))

(fn `UserConstructionScript`)